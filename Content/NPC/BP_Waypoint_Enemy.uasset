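; Enemy NPC that patrols an array of waypoints in an endless loop and shows a floating health bar.
; BeginPlay starts an AIMoveTo loop that advances and wraps the waypoint index after each success, with no failure handling.
; Tick updates the bar from the health component and turns it toward the player camera.
; Health changes are only printed; sight and death handlers are empty, and a random-roam event is never run.
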(event OnSeePawn(PawnSensing)
  (params (Pawn :type Pawn%20Object%20Reference)))

(event OnHealthDepleted(BP_HealthComponent))

(event OnHealthChanged(BP_HealthComponent)
  (params (NewHealth :type Float%20%28double-precision%29))
  (Development|PrintString (Utilities|String|Append "NewHealth" (Utilities|String|ToString(Float) NewHealth))))

(event Custom|BeginPatrol
  (bind _waypoints (Variables|Default|GetWaypoints))
  (AI|AIMoveTo self "0, 0, 0" (Utilities|Array|Get(acopy) _waypoints (Variables|Default|GetCurrent%20Waypoint)) 5.0 false :!label _label
    (:OnSuccess
      (Math|Integer|IncrementInt (Variables|Default|GetCurrent%20Waypoint)
        (:%20%20
          (if (>= (Variables|Default|GetCurrent%20Waypoint) (Utilities|Array|Length _waypoints))
            (Variables|Default|SetCurrent%20Waypoint 0))
          (Utilities|FlowControl|Delay 0.2)
          (goto _label))))))

(event Custom|MoveRandom
  (AI|AIMoveTo self (.RandomLocation (AI|Navigation|GetRandomReachablePointinRadius (Transformation|GetActorLocation) 3e+03 0 0)) 0 5.0 false :!label _label
    (:then
      (Utilities|FlowControl|Delay 1.0)
      (goto _label))))

(event EventBeginPlay
  (CallFunction|BeginPatrol))

(event EventTick
  (params (DeltaSeconds :type Float%20%28single-precision%29))
  (bind _health_bar (Variables|Default|GetHealth%20Bar))
  (bind _bp_healthcomponent (Variables|Default|GetBP_HealthComponent))
  (bind _ashealth_bar (Utilities|Casting|CastToHealth_Bar (UserInterface|GetWidget (Variables|Default|GetHealth%20Bar))))
  (Progress|SetPercent (Variables|/Game/Components/Health_Bar.Health_Bar_C|GetHealthBar _ashealth_bar) (/ (Variables|/Game/Components/BP_HealthComponent.BP_HealthComponent_C|GetHealth _bp_healthcomponent) (Variables|/Game/Components/BP_HealthComponent.BP_HealthComponent_C|GetMaxHealth _bp_healthcomponent)))
  (Transformation|SetWorldRotation _health_bar (Math|Rotator|FindLookatRotation (Transformation|GetWorldLocation _health_bar) (Transformation|GetWorldLocation (Variables|/Script/Engine.Actor|GetRootComponent (Game|GetPlayerCameraManager 0)))) false false))

(fn ConstructionScript)